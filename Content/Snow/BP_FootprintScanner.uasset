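; BP_FootprintScanner is a volume actor that leaves snow footprint decals under characters moving inside its box.
; A looping timer polls the box for overlapping Mordhau characters every fraction of a second.
; Each one moving on the ground above a minimum horizontal speed gets a temporary downward-projected decal at its right footstep socket, aligned to the actor's yaw.
; Prints follow the timer rather than animation footfalls, and only the right-foot socket is used.
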(event EventBeginPlay
  (Utilities|Time|SetTimerbyFunctionName 0 "CheckFootstep" 0.3 true))

(fn ConstructionScript)

(fn CheckFootstep
  (for _array_element (Collision|GetOverlappingActors (Variables|Default|GetBox) "/Game/Mordhau/Blueprints/Characters/BP_MordhauCharacter.BP_MordhauCharacter_C" :!class /Script/Engine.PrimitiveComponent)
    (if (AI|Components|NavMovement|IsMovingonGround (Variables|/Script/Engine.Character|GetCharacterMovement (.AsMordhau%20Character (Utilities|Casting|CastToMordhauCharacter _array_element))))
      (if (> (Math|Vector|VectorLengthXY (Transformation|GetVelocity (.AsMordhau%20Character (Utilities|Casting|CastToMordhauCharacter _array_element)))) 1e+02)
        (Rendering|Decal|SpawnDecalatLocation "/BRExtraMapsVanilla/Snow/DM_Footstep_Snow.DM_Footstep_Snow" "18.000000,25.000000,29.000000" (Transformation|GetSocketLocation (Variables|/Script/Engine.Character|GetMesh (.AsMordhau%20Character (Utilities|Casting|CastToMordhauCharacter _array_element))) "RightFootstep") (Math|Rotator|MakeRotator 0.0 -9e+01 (+ (.yaw (Transformation|GetActorRotation (.AsMordhau%20Character (Utilities|Casting|CastToMordhauCharacter _array_element)))) 9e+01)) 6e+01)))))